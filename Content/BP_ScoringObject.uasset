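; BP_ScoringObject is an actor with a Box trigger, apparently a placeholder for scoring when a character passes it while airborne.
; On actor begin overlap and Box end overlap, it gets the other actor's character movement through a GetCharacterMovementMessage call and checks it is valid.
; If that movement is falling, it only prints a debug string for entry or exit; no score is tracked yet.
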(event OnComponentEndOverlap(Box)
  (params (OverlappedComponent :type Primitive%20Component%20Object%20Reference) (OtherActor :type Actor%20Object%20Reference) (OtherComp :type Primitive%20Component%20Object%20Reference) (OtherBodyIndex :type Integer))
  (bind _outcharactermovementcomponent (Class|BPISkating|GetCharacterMovement(Message) OtherActor))
  (Utilities|IsValid _outcharactermovementcomponent
    (:Is%20Valid
      (if (AI|Components|NavMovement|IsFalling _outcharactermovementcomponent)
        (Development|PrintString "Passei")))))

(event EventBeginPlay)

(event Collision|EventActorBeginOverlap
  (params (OtherActor :type Actor%20Object%20Reference))
  (bind _outcharactermovementcomponent (Class|BPISkating|GetCharacterMovement(Message) OtherActor))
  (Utilities|IsValid _outcharactermovementcomponent
    (:Is%20Valid
      (if (AI|Components|NavMovement|IsFalling _outcharactermovementcomponent)
        (Development|PrintString "Hello")))))

(event EventTick
  (params (DeltaSeconds :type Float%20%28single-precision%29)))

(fn ConstructionScript)