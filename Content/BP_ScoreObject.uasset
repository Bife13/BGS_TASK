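; BP_ScoreObject is an actor with a box component that reports where an overlapping actor sits along the box's right axis.
; Actor begin overlap and box end overlap both call NewFunction, which prints the dot product of the actor-to-box offset and the box's right vector.
; Despite the name, it keeps no score, only printing debug output.
; Disconnected nodes hold unused character-falling checks with debug prints.
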(event OnComponentEndOverlap(BoxComponent)
  (params (OverlappedComponent :type Primitive%20Component%20Object%20Reference) (OtherActor :type Actor%20Object%20Reference) (OtherComp :type Primitive%20Component%20Object%20Reference) (OtherBodyIndex :type Integer))
  (CallFunction|NewFunction OtherActor))

(event EventBeginPlay)

(event Collision|EventActorBeginOverlap
  (params (OtherActor :type Actor%20Object%20Reference))
  (CallFunction|NewFunction OtherActor))

(event EventTick
  (params (DeltaSeconds :type Float%20%28single-precision%29)))

(fn ConstructionScript)

(fn NewFunction
  (params (self2 :type Actor%20Object%20Reference))
  (bind _boxcomponent (Variables|Default|GetBoxComponent))
  (Development|PrintString (Utilities|String|ToString(Float) (Math|Vector|DotProduct (- (Transformation|GetWorldLocation _boxcomponent) (Transformation|GetActorLocation self2)) (Math|Vector|GetRightVector _boxcomponent)))))